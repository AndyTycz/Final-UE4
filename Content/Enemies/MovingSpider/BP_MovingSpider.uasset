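; Moving spider enemy that chases the player and attacks in melee, overriding its parent's roaming with an empty event.
; In combat, it picks an attack by distance, waits, then uses AI MoveTo before attacking or clearing its target.
; Tick yaws it toward the player except during the brief charge window.
; Heavy and Special attacks use forward sphere overlaps to damage and launch the hero, and death uses a montage and physics ragdoll.
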(event `/Game/Enemies/MovingSpider/BPI_EnemyAI.SetRoaming`)

(event `self.ReceiveTick`
  (params (DeltaSeconds :type "Float (single-precision)"))
  (bind _newparam (`self.GetPlayerTarget`))
  (bind (_returnvalue_roll _returnvalue_pitch _returnvalue_yaw) (`KismetMathLibrary.BreakRotator` (`KismetMathLibrary.FindLookAtRotation` (`self.K2_GetActorLocation`) (`self.K2_GetActorLocation` _newparam))))
  ;[1 1 1] Override Tick so we don't rotate while charge
  (if (and (`self.GetCombatState`) (not (`self.bIsCharging`)) (not (`self.GetIsDead`)))
    (`/Engine/EditorBlueprintResources/StandardMacros.IsValid` _newparam
      (:`Is Valid`
        (`self.K2_SetActorRotation` (`KismetMathLibrary.MakeRotator` 0.0 0.0 _returnvalue_yaw))))))

(event `/Game/Enemies/MovingSpider/BPI_EnemyAI.ChasePlayer`
  ;[1 1 1] Chase Player
  (if (and (`self.GetCombatState`) (not (`self.GetIsDead`)))
    (bind _lenght (`self.PickAttack` (`self.GetDistanceTo` self (`self.GetPlayerTarget`))))
    (`KismetSystemLibrary.Delay` (+ _lenght 0.5))
    (`|AIMoveTo` self (0.0 0.0 0.0) (`self.GetPlayerTarget`) 150.0 true
      (:`OnSuccess`
        (`/Game/Enemies/MovingSpider/BPI_EnemyAI.DoAttackChoices`))
      (:`OnFail`
        (`/Game/Enemies/MovingSpider/BPI_EnemyAI.ClearTarget`)))))

(event `/Game/Enemies/MovingSpider/BPI_EnemyAI.DoSphereOverlap`
  ;[1 1 1] Heavy Attack with Knockback
  (switch `/Game/Enemies/MovingSpider/E_AIAttackTypes` (`self.GetAttackType`)
    (:`NewEnumerator1`
      (bind _outactors (`KismetSystemLibrary.SphereOverlapActors` (+ (`self.K2_GetActorLocation`) (* (`self.GetActorForwardVector`) 250)) 100.0 (`|MakeArray` "ObjectTypeQuery3" :!type "EObjectTypeQuery Enum") null (`|MakeArray` self :!type "Actor Object Reference")))
      (for _array_element _outactors
        (bind _asbp_hero_character (cast `/Game/Character/BP_HeroCharacter` _array_element))
        (`self.GetDamage` _asbp_hero_character)
        (`self.LaunchCharacter` _asbp_hero_character (* (`KismetMathLibrary.MakeVector` (.x (`KismetMathLibrary.GetDirectionUnitVector` (`self.K2_GetActorLocation`) (`self.K2_GetActorLocation` _asbp_hero_character))) (.y (`KismetMathLibrary.GetDirectionUnitVector` (`self.K2_GetActorLocation`) (`self.K2_GetActorLocation` _asbp_hero_character))) (+ (.z (`KismetMathLibrary.GetDirectionUnitVector` (`self.K2_GetActorLocation`) (`self.K2_GetActorLocation` _asbp_hero_character))) 1.0)) 500.0) false false)
        (`GameplayStatics.PlaySound2D` (`self.PlayerHitSound`) 1.0 1.0 0.0 null null)))))

(event `/Game/Enemies/MovingSpider/BPI_EnemyAI.DoChargeOverlap`
  ;[1 1 1] Charge Attack
  (switch `/Game/Enemies/MovingSpider/E_AIAttackTypes` (`self.GetAttackType`)
    (:`NewEnumerator3`
      (set `self.bIsCharging` true)
      (`KismetSystemLibrary.Delay` 0.2)
      (bind _outactors (`KismetSystemLibrary.SphereOverlapActors` (+ (`self.K2_GetActorLocation`) (* (`self.GetActorForwardVector`) 200)) 100.0 (`|MakeArray` "ObjectTypeQuery3" :!type "EObjectTypeQuery Enum") null (`|MakeArray` self :!type "Actor Object Reference")))
      (set `self.bIsCharging` false)
      (for _array_element _outactors
        (bind _asbp_hero_character (cast `/Game/Character/BP_HeroCharacter` _array_element))
        (`self.GetDamage` _asbp_hero_character)
        (`self.LaunchCharacter` _asbp_hero_character (* (`KismetMathLibrary.MakeVector` (.x (`KismetMathLibrary.GetDirectionUnitVector` (`self.K2_GetActorLocation`) (`self.K2_GetActorLocation` _asbp_hero_character))) (.y (`KismetMathLibrary.GetDirectionUnitVector` (`self.K2_GetActorLocation`) (`self.K2_GetActorLocation` _asbp_hero_character))) (+ (.z (`KismetMathLibrary.GetDirectionUnitVector` (`self.K2_GetActorLocation`) (`self.K2_GetActorLocation` _asbp_hero_character))) 1.0)) 400.0) false false)
        (`GameplayStatics.PlaySound2D` (`self.PlayerHitSound`) 1.0 1.0 0.0 null null)))))

(fn `DoRagdoll`
  (bind _mesh (`self.Mesh`))
  (`PrimitiveComponent.SetCollisionEnabled` _mesh "QueryAndPhysics")
  (`SkeletalMeshComponent.SetAllBodiesSimulatePhysics` _mesh true)
  (`SkeletalMeshComponent.SetAllBodiesPhysicsBlendWeight` _mesh 1.0 false))

(fn `PlayDeathAnimation`
  (`self.Play_Montage` (`self.Mesh`) "/Game/Enemies/MovingSpider/Spider_DeathMontage.Spider_DeathMontage"))

(fn `UserConstructionScript`
  (`parent.UserConstructionScript`))