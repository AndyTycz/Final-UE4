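; Suicide-bomber enemy that chases the hero and explodes.
; Sighting updates the AI blackboard and raises speed in two stages, then ignites body fire and a long scream.
; It explodes with radial damage when the scream ends, or direct damage on hero overlap, then OnDeath ragdolls it and Tick destroys it after a delay.
; Taking damage stops movement and plays a random death montage without calling OnDeath.
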(event `self.ReceiveBeginPlay`
  (set `CharacterMovementComponent.MaxWalkSpeed` (`self.WalkSpeed`) (`self.CharacterMovement`)))

(event `self.AIPerception.OnTargetPerceptionUpdated`
  (params (Actor :type "Actor Object Reference") (Stimulus :type "AIStimulus Structure"))
  (bind (_age _expirationage _strength _stimuluslocation _receiverlocation _tag _bsuccessfullysensed) (break `AIStimulus` Stimulus))
  (bind _charactermovement (`self.CharacterMovement`))
  ;[1 1 1] Saw and chase player
  (bind _asbp_hero_character (cast `/Game/Character/BP_HeroCharacter` Actor))
  (if (not (`|EnumEquality` (`HeroCharacter.movementType` _asbp_hero_character) "EMType_Death"))
    (`BlackboardComponent.SetValueAsBool` (`AIBlueprintHelperLibrary.GetBlackboard` null) "bSeesPlayer" _bsuccessfullysensed)
    (if _bsuccessfullysensed
      (set `CharacterMovementComponent.MaxWalkSpeed` (`self.ChasePlayerSpeed`) _charactermovement)
      (`KismetSystemLibrary.Delay` 2.0)
      (set `CharacterMovementComponent.MaxWalkSpeed` (`self.MaxChaseSpeed`) _charactermovement)
      (if (not (`self.bDed`))
        (`ActorComponent.Activate` (`self.Full Body Fire`) false)
        (`ActorComponent.Activate` (`self.LongScream_Cue`) false)))))

(event `self.ReceiveTick`
  (params (DeltaSeconds :type "Float (single-precision)"))
  ;[1 1 1] Death
  (if (`self.bDed`)
    (`BlackboardComponent.SetValueAsBool` (`AIBlueprintHelperLibrary.GetBlackboard` null) "isDead" false)
    (`KismetSystemLibrary.Delay` 2.0)
    (`ActorComponent.Deactivate` (`self.Full Body Fire`))
    (`ActorComponent.Deactivate` (`self.BombFire`))
    (`self.K2_DestroyActor`)))

(event `self.LongScream_Cue.OnAudioFinished`
  ;[1 1 1] Explode After big scream
  (if (not (`self.bDed`))
    (`GameplayStatics.ApplyRadialDamage` :`BaseDamage` 25.0 :`Origin` (`KismetMathLibrary.Conv_DoubleToVector` (`SkeletalMeshComponent.GetPosition` (`self.Mesh`))) :`DamageRadius` 120.0 :`DamageTypeClass` "/Script/Engine.DamageType" :`DamageCauser` null :`InstigatedByController` null)
    (`ActorComponent.Activate` (`self.BOOOM`) false)
    (`ActorComponent.Activate` (`self.ExplosionSound`) false)
    (`self.OnDeath`)))

(event `self.ReceiveAnyDamage`
  (params (Damage :type "Float (single-precision)") (DamageType :type "DamageType Object Reference") (InstigatedBy :type "Controller Object Reference") (DamageCauser :type "Actor Object Reference"))
  ;[1 1 1] Choose death animation
  (if (not (`self.bDed`))
    (`BlackboardComponent.SetValueAsBool` (`AIBlueprintHelperLibrary.GetBlackboard` null) "isDead" false)
    (`CharacterMovementComponent.DisableMovement` (`self.CharacterMovement`))
    (if (<= (`KismetMathLibrary.RandomFloat`) 0.5)
      (`self.PlayAnimMontage` "/Game/Enemies/Sploder/DeathMontage.DeathMontage" 1.0 "Death01")
      (else
        (`self.PlayAnimMontage` "/Game/Enemies/Sploder/DeathMontage.DeathMontage" 1.0 "Death02")))))

(event `self.Boom collider.OnComponentBeginOverlap`
  (params (OverlappedComponent :type "PrimitiveComponent Object Reference") (OtherActor :type "Actor Object Reference") (OtherComp :type "PrimitiveComponent Object Reference") (OtherBodyIndex :type Integer) (bFromSweep :type Boolean) (SweepResult :type "HitResult Structure (by ref)"))
  (bind _asbp_hero_character (cast `/Game/Character/BP_HeroCharacter` OtherActor))
  (`GameplayStatics.ApplyDamage` _asbp_hero_character (`self.ExplosionDamage`) null null "/Script/Engine.DamageType")
  (`ActorComponent.Activate` (`self.ExplosionSound`) false)
  (`ActorComponent.Activate` (`self.BOOOM`) false)
  (`PrimitiveComponent.SetCollisionEnabled` (`self.Boom collider`) "NoCollision")
  (`PrimitiveComponent.SetCollisionEnabled` (`self.CapsuleComponent`) "NoCollision")
  (`self.OnDeath`))

(fn `OnDeath`
  (bind _mesh (`self.Mesh`))
  (`ActorComponent.Deactivate` (`self.Full Body Fire`))
  (`ActorComponent.Deactivate` (`self.BombFire`))
  (`ActorComponent.Deactivate` (`self.LongScream_Cue`))
  (`PrimitiveComponent.SetCollisionEnabled` _mesh "QueryAndPhysics")
  (`SkeletalMeshComponent.SetAllBodiesSimulatePhysics` _mesh true)
  (`SkeletalMeshComponent.SetAllBodiesPhysicsBlendWeight` _mesh 1.0 false)
  (set `self.bDed` true))

(fn `UserConstructionScript`)