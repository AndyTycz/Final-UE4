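; Base enemy AI character that roams near its spawn, fights BP_HeroCharacter and dies at zero health.
; SetPlayerTarget starts combat: optional distance-based taunt, then an AIMoveTo chase-and-attack loop, with a timer clearing distant targets.
; Random montages play for light, heavy or special attacks, picked by distance and chance.
; The attack type sets damage for melee-sphere and forward-overlap hits; PlayDeathAnimation is an empty stub.
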(event `self.ReceiveBeginPlay`
  ;[1 1 1] Set Starting Movement State
  (set `self.StartingLocation` (`self.K2_GetActorLocation`))
  (`KismetSystemLibrary.Delay` 2.0)
  (`self.SetRoaming`))

(event `Play_Montage`
  (params (InSkeletalMeshComponent :type "SkeletalMeshComponent Object Reference") (MontageToPlay :type "AnimMontage Object Reference") (StartingSection :type Name))
  (`|PlayMontage` InSkeletalMeshComponent MontageToPlay 1.0 0.0 StartingSection))

(event `self.ReceiveAnyDamage`
  (params (Damage :type "Float (single-precision)") (DamageType :type "DamageType Object Reference") (InstigatedBy :type "Controller Object Reference") (DamageCauser :type "Actor Object Reference"))
  (bind _health (`self.Health`))
  ;[1 1 1] TakeDamage
  (set `self.Health` (- _health Damage))
  (`GameplayStatics.PlaySound2D` (`self.GotHitSound`) 1.0 1.0 0.0 null null)
  (if (<= _health 0.0)
    (`self.Death`)))

(event `self.SetRoaming`
  ;[1 1 1] Roam Around Starting Position
  (if (and (not (`self.bIsRoaming`)) (not (`self.bIsCombat`)))
    (`self.MovementState` "NewEnumerator1")
    (`|AIMoveTo` self (`NavigationSystemV1.K2_GetRandomReachablePointInRadius` (`self.StartingLocation`) 1000.0 null null) null
      (:`then`
        (set `self.bIsRoaming` true))
      (:`OnSuccess`
        (set `self.bIsRoaming` false)
        (`KismetSystemLibrary.Delay` 4.0))
      (:`OnFail`
        (`self.ClearTarget`)))))

(event `self.SetPlayerTarget`
  (params (Target :type "Actor Object Reference"))
  ;[1 1 1] Set Player Target and Follow w/ chase
  (set `self.PlayerTarget` Target)
  (set `self.bIsCombat` true)
  (set `self.bIsRoaming` false)
  (`self.SetActorTickEnabled` true)
  (set `self.StartCombatLocation` (`self.K2_GetActorLocation`))
  (`self.MovementState` "NewEnumerator2")
  (`self.CheckForTaunt`)
  (bind _returnvalue (`KismetSystemLibrary.K2_SetTimer` null "PlayerDistanceCheck" 0.5 true))
  (set `self.DistanceHandle` _returnvalue))

(event `self.Death`
  (bind _charactermovement (`self.CharacterMovement`))
  ;[1 1 1] Death
  (if (not (`self.bIsDead`))
    (set `self.bIsDead` true)
    (`self.PlayDeathAnimation`)
    (`self.DetachFromControllerPendingDestroy`)
    (`PrimitiveComponent.SetCollisionEnabled` (`self.CapsuleComponent`) "NoCollision")
    (`CharacterMovementComponent.SetAvoidanceEnabled` _charactermovement true)
    (`CharacterMovementComponent.DisableMovement` _charactermovement)
    (`KismetSystemLibrary.Delay` 10.0)
    (`self.K2_DestroyActor`)))

(event `self.ReceiveTick`
  (params (DeltaSeconds :type "Float (single-precision)"))
  ;[1 1 1] Set Player Target and Follow w/ chase
  (if (and (`self.bIsCombat`) (not (`self.bIsDead`)))
    (bind _playertarget (`self.PlayerTarget`)
      (:`then`
        (bind (_returnvalue_roll _returnvalue_pitch _returnvalue_yaw) (`KismetMathLibrary.BreakRotator` (`KismetMathLibrary.FindLookAtRotation` (`self.K2_GetActorLocation`) (`self.K2_GetActorLocation` _playertarget))))
        (`self.K2_SetActorRotation` (`KismetMathLibrary.MakeRotator` 0.0 0.0 _returnvalue_yaw)))
      (:`else`))))

(event `self.ClearTarget`
  ;[1 1 1] Clear Target and reset roaming
  (set `self.bIsCombat` false)
  (`self.SetActorTickEnabled` false)
  (set `self.PlayerTarget` null)
  (`/Game/Enemies/AI_EnemyBase.Clear Target` (cast `/Game/Enemies/AI_EnemyBase` (`self.GetController`) :!pure true))
  (`|AIMoveTo` self (`self.StartCombatLocation`) null
    (:`OnSuccess`
      (`self.SetRoaming`))
    (:`OnFail`
      (`self.K2_SetActorLocation` (`self.StartingLocation`))
      (`self.SetRoaming`))))

(event `self.ChasePlayer`
  ;[1 1 1] Chase Player
  (if (and (`self.bIsCombat`) (not (`self.bIsDead`)))
    (`|AIMoveTo` self (0.0 0.0 0.0) (`self.PlayerTarget`) 150.0 true
      (:`OnSuccess`
        (`self.DoAttackChoices`))
      (:`OnFail`
        (`self.ClearTarget`)))))

(event `self.CheckForTaunt`
  (bind _output (`self.GetMontage` (`self.TauntMontage`)))
  ;[1 1 1] Do Taunt animation if player is far away
  (if (not (`self.bIsDead`))
    (`Controller.StopMovement` (`self.GetController`))
    (if (>= (`self.GetDistanceTo` self (`self.PlayerTarget`)) (`self.DistanceToTaunt`))
      (`self.Play_Montage` (`self.Mesh`) _output)
      (`GameplayStatics.PlaySound2D` (`self.TauntSound`) 1.0 1.0 0.0 null null)
      (bind _returnvalue (`AnimSequenceBase.GetPlayLength` _output))
      (`KismetSystemLibrary.Delay` _returnvalue)
      (`self.ChasePlayer`)
      (else
        (`self.ChasePlayer`)))))

(event `self.DoAttackChoices`
  ;[1 1 1] Select Attack Variation
  (if (not (`self.bIsDead`))
    (bind _playertarget (`self.PlayerTarget`)
      (:`then`
        (bind _asbp_hero_character (cast `/Game/Character/BP_HeroCharacter` _playertarget))
        (if (`|EnumInequality` (`HeroCharacter.movementType` _asbp_hero_character) "EMType_Death")
          (bind _lenght (`self.PickAttack` (`self.GetDistanceTo` self (`self.PlayerTarget`))))
          (`KismetSystemLibrary.Delay` (+ _lenght 0.5))
          (`self.ChasePlayer`)
          (else
            (`self.ClearTarget`))))
      (:`else`))))

(event `self.SetMeleeCollision`
  (params (State :type Boolean))
  (bind _meleesphere (`self.MeleeSphere`))
  ;[1 1 1] AnimNotif Activate collision
  (if State
    (`PrimitiveComponent.SetCollisionEnabled` _meleesphere "QueryOnly")
    (else
      (`PrimitiveComponent.SetCollisionEnabled` _meleesphere "NoCollision"))))

(event `self.MeleeSphere.OnComponentBeginOverlap`
  (params (OverlappedComponent :type "PrimitiveComponent Object Reference") (OtherActor :type "Actor Object Reference") (OtherComp :type "PrimitiveComponent Object Reference") (OtherBodyIndex :type Integer) (bFromSweep :type Boolean) (SweepResult :type "HitResult Structure (by ref)"))
  ;[1 1 1] Damage Overlappers
  (bind _asbp_hero_character (cast `/Game/Character/BP_HeroCharacter` OtherActor))
  (`self.GetDamage` _asbp_hero_character)
  (`GameplayStatics.PlaySound2D` (`self.PlayerHitSound`) 1.0 1.0 0.0 null null))

(event `self.DoSphereOverlap`
  ;[1 1 1] Damage Overlappers
  (`KismetSystemLibrary.SphereOverlapActors` (+ (`self.K2_GetActorLocation`) (* (`self.GetActorForwardVector`) 250)) 100.0 (`|MakeArray` "ObjectTypeQuery3" :!type "EObjectTypeQuery Enum") null (`|MakeArray` self :!type "Actor Object Reference"))
  (for _array_element _
    (bind _asbp_hero_character (cast `/Game/Character/BP_HeroCharacter` _array_element))
    (`self.GetDamage` _asbp_hero_character)
    (`GameplayStatics.PlaySound2D` (`self.PlayerHitSound`) 1.0 1.0 0.0 null null)))

(fn `AttackPercentage`
  (params (Percent :type "Float (double-precision)"))
  (returns (Return :type Boolean))
  (return (select `bool` (== Percent 0.0) :`false` (<= (`KismetMathLibrary.RandomFloatInRange` 0.0 100.0) Percent))))

(fn `GetAttackType`
  (returns (AttackTypes :type "/Game/Enemies/MovingSpider/E_AIAttackTypes Enum"))
  (return (`self.AttackTypes`)))

(fn `GetCombatState`
  (returns (bIsCombat :type Boolean))
  (return (`self.bIsCombat`)))

(fn `GetDamage`
  (params (HitPlayer :type "Actor Object Reference"))
  (switch `/Game/Enemies/MovingSpider/E_AIAttackTypes` (`self.AttackTypes`)
    (:`NewEnumerator0`
      (`GameplayStatics.ApplyDamage` HitPlayer (`self.LightAttackDamage`) null self "/Script/Engine.DamageType"))
    (:`NewEnumerator1`
      (`GameplayStatics.ApplyDamage` HitPlayer (`self.HeavyAttackDamage`) null self "/Script/Engine.DamageType"))
    (:`NewEnumerator3`
      (`GameplayStatics.ApplyDamage` HitPlayer (`self.SpecialAttackDamage`) null self "/Script/Engine.DamageType"))))

(fn `GetIsDead`
  (returns (bIsDead :type Boolean))
  (return (`self.bIsDead`)))

(fn `GetMontage`
  (params (AttackMontages :type "Array of AnimMontage Object Reference"))
  (returns (Output :type "AnimMontage Object Reference"))
  (return (`|GetArrayItem` AttackMontages (`KismetMathLibrary.RandomIntegerInRange` 0 (- (`KismetArrayLibrary.Array_Length` AttackMontages) 1)))))

(fn `GetPlayerTarget`
  (returns (NewParam :type "Actor Object Reference"))
  (return (`self.PlayerTarget`)))

(fn `GetSetStartingSpawn`
  (params (StartingLocation :type "Vector Structure"))
  (returns (Output_Get :type "Vector Structure"))
  (bind _output_get (set `self.StartingLocation` StartingLocation))
  (return _output_get))

(fn `GetSightRadius`
  (returns (Radius :type "Float (double-precision)"))
  (return (`self.SightRadius`)))

(fn `MovementState`
  (params (State :type "/Game/Enemies/MovingSpider/E_AIMovementStates Enum" :default "NewEnumerator0"))
  (bind _walkspeed (`self.WalkSpeed`))
  (set `CharacterMovementComponent.MaxWalkSpeed` (select `/Game/Enemies/MovingSpider/E_AIMovementStates` State :`NewEnumerator1` _walkspeed :`NewEnumerator2` (* _walkspeed (`self.SpeedMultiplier`))) (`self.CharacterMovement`)))

(fn `PickAttack`
  (params (DistanceToPlayer :type "Float (double-precision)"))
  (returns (Lenght :type "Float (double-precision)"))
  (bind _output (`self.GetMontage` (`self.LightAttackMontages`)))
  (bind _output_2 (`self.GetMontage` (`self.HeavyAttackMontages`)))
  (bind _output_3 (`self.GetMontage` (`self.SpecialAttackMontages`)))
  (if (<= DistanceToPlayer (`self.MeleeDistance`))
    (if (`self.AttackPercentage` (`self.Light Attack Chance`))
      (set `self.AttackTypes` "NewEnumerator0")
      (`self.Play_Montage` (`self.Mesh`) _output)
      (bind _returnvalue (`AnimSequenceBase.GetPlayLength` _output))
      (return _returnvalue)
      (else
        (set `self.AttackTypes` "NewEnumerator1")
        (`self.Play_Montage` (`self.Mesh`) _output_2)
        (bind _returnvalue_2 (`AnimSequenceBase.GetPlayLength` _output_2))
        (return _returnvalue_2)))
    (else
      (set `self.AttackTypes` "NewEnumerator3")
      (`self.Play_Montage` (`self.Mesh`) _output_3)
      (bind _returnvalue_3 (`AnimSequenceBase.GetPlayLength` _output_3))
      (return _returnvalue_3))))

(fn `PlayDeathAnimation`)

(fn `PlayerDistanceCheck`
  (bind _returnvalue (`self.GetDistanceTo` self (`self.PlayerTarget`)))
  (`KismetSystemLibrary.PrintString` (`KismetStringLibrary.Conv_DoubleToString` _returnvalue))
  (if (>= _returnvalue 2500.0)
    (`self.ClearTarget`)
    (`KismetSystemLibrary.K2_ClearAndInvalidateTimerHandle` (`self.DistanceHandle`))))

(fn `UserConstructionScript`)