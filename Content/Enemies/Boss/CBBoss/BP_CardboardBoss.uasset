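; Cardboard boss enemy that chases and attacks the hero once SetPlayerTarget starts combat.
; DefaultChase loops AI movement into one of three random montages, toggling Tick so the boss turns toward the hero during attacks.
; Separate hit events use sphere overlaps for slam, punch and special damage, some adding knockback, alongside an effects helper.
; The entrance sequence leading to FirstChase and a distance-check timer are left unwired.
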(event `self.ReceiveBeginPlay`
  (`self.GetSetStartingSpawn` (`self.K2_GetActorLocation`))
  (`KismetSystemLibrary.Delay` 2.0))

(event `/Game/Enemies/MovingSpider/BPI_EnemyAI.SetPlayerTarget`
  (params (Target :type "Actor Object Reference"))
  (bind _output_get (set `self.PlayerTarget` Target))
  (bind _asbp_hero_character (cast `/Game/Character/BP_HeroCharacter` _output_get))
  (set `/Game/Character/BP_HeroCharacter.bHeroCanMove` true _asbp_hero_character)
  (set `self.bIsCombat` true)
  (set `self.StartCombatLocation` (`self.K2_GetActorLocation`))
  (`self.MovementState` "NewEnumerator1")
  (`self.DefaultChase`))

(event `self.ReceiveTick`
  (params (DeltaSeconds :type "Float (single-precision)"))
  (if (and (`self.bIsCombat`) (not (`self.bIsDead`)))
    (bind _playertarget (`self.PlayerTarget`)
      (:`then`
        (bind (_returnvalue_roll _returnvalue_pitch _returnvalue_yaw) (`KismetMathLibrary.BreakRotator` (`KismetMathLibrary.FindLookAtRotation` (`self.K2_GetActorLocation`) (`self.K2_GetActorLocation` _playertarget))))
        (`self.K2_SetActorRotation` (`KismetMathLibrary.MakeRotator` 0.0 0.0 _returnvalue_yaw)))
      (:`else`))))

(event `DefaultChase`
  ;[1 1 1] Chase And Pick Attack
  (`|AIMoveTo` self (0.0 0.0 0.0) (`self.PlayerTarget`) 250.0 true
    (:`OnSuccess`
      (`self.SetActorTickEnabled` true)
      (switch `int` (`KismetMathLibrary.RandomIntegerInRange` 0 2)
        (:`0`
          (`|PlayMontage` (`self.Mesh`) "/Game/Enemies/Boss/Boss_SwingAndSlamMontage.Boss_SwingAndSlamMontage" 1.3
            (:`OnCompleted`
              _)))
        (:`1`
          (`|PlayMontage` (`self.Mesh`) "/Game/Enemies/Boss/Boss_ComboAttackMontage.Boss_ComboAttackMontage" 1.2
            (:`OnCompleted`
              _)))
        (:`2`
          (`|PlayMontage` (`self.Mesh`) "/Game/Enemies/Boss/Boss_Attack01Montage.Boss_Attack01Montage" 1.3
            (:`OnCompleted`
              _))))
      (`self.SetActorTickEnabled` false)
      (`self.DefaultChase`))))

(event `PlayEntranceMontage`
  (params (InSkeletalMeshComponent :type "SkeletalMeshComponent Object Reference") (MontageToPlay :type "AnimMontage Object Reference"))
  ;[1 1 1] Initial chase and slap
  (`|PlayMontage` InSkeletalMeshComponent MontageToPlay
    (:`OnCompleted`
      (`self.FirstChase`)
      (bind _asbp_hero_character (cast `/Game/Character/BP_HeroCharacter` (`self.GetPlayerTarget`)))
      (set `/Game/Character/BP_HeroCharacter.bHeroCanMove` true _asbp_hero_character))))

(event `FirstChase`
  ;[1 1 1] Initial chase and slap
  (`|AIMoveTo` self (0.0 0.0 0.0) (`self.PlayerTarget`) 700.0 true
    (:`OnSuccess`
      (`self.FirstAttack` (`self.Mesh`) "/Game/Enemies/Boss/Boss_FirstAttackMontage.Boss_FirstAttackMontage"))
    (:`OnFail`
      (`/Game/Enemies/MovingSpider/BPI_EnemyAI.ClearTarget`))))

(event `FirstAttack`
  (params (InSkeletalMeshComponent :type "SkeletalMeshComponent Object Reference") (MontageToPlay :type "AnimMontage Object Reference"))
  ;[1 1 1] Initial chase and slap
  (`|PlayMontage` InSkeletalMeshComponent MontageToPlay
    (:`OnCompleted`
      (`self.DefaultChase`))))

(event `/Game/Enemies/Boss/BPI_BossEnemies.GroundSlam`
  (params (Location :type "Vector Structure"))
  ;[1 1 1] Bonk damage attack
  (bind (_outactors _returnvalue) (`KismetSystemLibrary.SphereOverlapActors` Location 200.0 (`|MakeArray` "ObjectTypeQuery3" :!type "EObjectTypeQuery Enum") "/Game/Character/BP_HeroCharacter.BP_HeroCharacter_C"))
  (if _returnvalue
    (for _array_element _outactors
      (`GameplayStatics.ApplyDamage` _array_element 40.0 null self "/Script/Engine.DamageType"))))

(event `/Game/Enemies/Boss/BPI_BossEnemies.BossVFX`
  (params (VFX :type "ParticleSystem Object Reference") (Location :type "Vector Structure") (Rotation :type "Rotator Structure") (Scale :type "Vector Structure") (Sound :type "SoundCue Object Reference"))
  ;[1 1 1] Bonk
  (`GameplayStatics.SpawnEmitterAtLocation` VFX Location Rotation Scale)
  (`GameplayStatics.PlaySoundAtLocation` Sound Location (struct) 1.0 1.0 0.0 null null null))

(event `/Game/Enemies/Boss/BPI_BossEnemies.Attack01Punch`
  ;[1 1 1] FistAttack
  (bind _outactors (`KismetSystemLibrary.SphereOverlapActors` (+ (`self.K2_GetActorLocation`) (* (`self.GetActorForwardVector`) 200.0)) 150.0 (`|MakeArray` "ObjectTypeQuery3" :!type "EObjectTypeQuery Enum") "/Game/Character/BP_HeroCharacter.BP_HeroCharacter_C"))
  (for _array_element _outactors
    (bind _asbp_hero_character (cast `/Game/Character/BP_HeroCharacter` _array_element))
    (`self.LaunchCharacter` _asbp_hero_character (* (`KismetMathLibrary.MakeVector` (.x (`KismetMathLibrary.GetDirectionUnitVector` (`self.K2_GetActorLocation`) (`self.K2_GetActorLocation` _asbp_hero_character))) (.y (`KismetMathLibrary.GetDirectionUnitVector` (`self.K2_GetActorLocation`) (`self.K2_GetActorLocation` _asbp_hero_character))) (+ (.z (`KismetMathLibrary.GetDirectionUnitVector` (`self.K2_GetActorLocation`) (`self.K2_GetActorLocation` _asbp_hero_character))) 1.0)) 400.0) false false)
    (`GameplayStatics.PlaySound2D` (`self.PlayerHitSound`) 1.0 1.0 0.0 null null)
    (`GameplayStatics.ApplyDamage` _asbp_hero_character (`self.LightAttackDamage`) null null "/Script/Engine.DamageType")))

(event `/Game/Enemies/Boss/BPI_BossEnemies.Attack01`
  ;[1 1 1] Attack After Fist
  (bind _outactors (`KismetSystemLibrary.SphereOverlapActors` (+ (`self.K2_GetActorLocation`) (* (`self.GetActorForwardVector`) 200.0)) 150.0 (`|MakeArray` "ObjectTypeQuery3" :!type "EObjectTypeQuery Enum") "/Game/Character/BP_HeroCharacter.BP_HeroCharacter_C"))
  (for _array_element _outactors
    (bind _asbp_hero_character (cast `/Game/Character/BP_HeroCharacter` _array_element))
    (`GameplayStatics.PlaySound2D` (`self.PlayerHitSound`) 1.0 1.0 0.0 null null)
    (`GameplayStatics.ApplyDamage` _asbp_hero_character (`self.LightAttackDamage`) null null "/Script/Engine.DamageType")))

(event `/Game/Enemies/Boss/BPI_BossEnemies.Attack02`
  (bind _returnvalue (+ (`self.K2_GetActorLocation`) (* (`self.GetActorForwardVector`) 200.0)))
  ;[1 1 1] Attack with knockback
  (bind _outactors (`KismetSystemLibrary.SphereOverlapActors` _returnvalue 150.0 (`|MakeArray` "ObjectTypeQuery3" :!type "EObjectTypeQuery Enum") "/Game/Character/BP_HeroCharacter.BP_HeroCharacter_C"))
  (`KismetSystemLibrary.DrawDebugSphere` _returnvalue 150.0 12 (struct :`R` 1.0 :`B` 1.0 :`A` 1.0) 2.0 2.0)
  (for _array_element _outactors
    (bind _asbp_hero_character (cast `/Game/Character/BP_HeroCharacter` _array_element))
    (`self.LaunchCharacter` _asbp_hero_character (* (`KismetMathLibrary.MakeVector` (.x (`KismetMathLibrary.GetDirectionUnitVector` (`self.K2_GetActorLocation`) (`self.K2_GetActorLocation` _asbp_hero_character))) (.y (`KismetMathLibrary.GetDirectionUnitVector` (`self.K2_GetActorLocation`) (`self.K2_GetActorLocation` _asbp_hero_character))) (+ (.z (`KismetMathLibrary.GetDirectionUnitVector` (`self.K2_GetActorLocation`) (`self.K2_GetActorLocation` _asbp_hero_character))) 1.5)) 400.0) false false)
    (`GameplayStatics.PlaySound2D` (`self.PlayerHitSound`) 1.0 1.0 0.0 null null)
    (`GameplayStatics.ApplyDamage` _asbp_hero_character (`self.SpecialAttackDamage`) null null "/Script/Engine.DamageType")))

(fn `UserConstructionScript`
  (`parent.UserConstructionScript`))