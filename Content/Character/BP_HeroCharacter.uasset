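; BP_HeroCharacter is the hero character Blueprint, with per-frame handling of movement lock and death.
; Tick switches capsule mobility between Static and Movable from HeroCanMove, using mobility as the freeze mechanism.
; When MovementType is death, Tick flags HeroDied, makes capsule and camera boom Static, enables pawn control rotation and changes camera field of view.
; BeginPlay is empty, and the background music node is unconnected.
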(event `self.ReceiveTick`
  (params (DeltaSeconds :type "Float (single-precision)"))
  (bind _cameraboom (`self.CameraBoom`))
  (if (not (`self.bHeroCanMove`))
    (`SceneComponent.SetMobility` (`self.CapsuleComponent`) "Static")
    (else
      (`SceneComponent.SetMobility` (`self.CapsuleComponent`) "Movable")))
  (if (`|EnumEquality` (`self.movementType`) "EMType_Death")
    (set `self.bHeroDied` true)
    (`SceneComponent.SetMobility` (`self.CapsuleComponent`) "Static")
    (`SceneComponent.SetMobility` _cameraboom "Static")
    (set `SpringArmComponent.bUsePawnControlRotation` true _cameraboom)
    (`CameraComponent.SetFieldOfView` (`self.FollowCamera`) 120.0)))

(event `self.ReceiveBeginPlay`)

(fn `UserConstructionScript`)