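; Main player controller Blueprint that adds animated transitions to the pause menu.
; It extends the parent's show and hide events, casting the inherited menu widget to PauseMenu to play its menu animation.
; Showing plays the animation forward; hiding plays it in reverse, then sets the widget hidden after a short fixed delay rather than waiting for the animation's finish event.
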(event `self.ShowPauseMenu`
  (`parent.ShowPauseMenu`)
  (bind _aspause_menu (cast `/Game/HUD/PauseMenu` (`self.pauseMenu`)))
  (`UserWidget.PlayAnimation` _aspause_menu (`/Game/HUD/PauseMenu.MenuAnimation` _aspause_menu) 0.0 1 "Forward" 1.0))

(event `self.HidePauseMenu`
  (`parent.HidePauseMenu`)
  (bind _aspause_menu (cast `/Game/HUD/PauseMenu` (`self.pauseMenu`)))
  (`UserWidget.PlayAnimation` _aspause_menu (`/Game/HUD/PauseMenu.MenuAnimation` _aspause_menu) 0.0 1 "Reverse" 1.0)
  (`KismetSystemLibrary.Delay` 0.25)
  (`Widget.SetVisibility` (`self.pauseMenu`) "Hidden"))

(fn `UserConstructionScript`)