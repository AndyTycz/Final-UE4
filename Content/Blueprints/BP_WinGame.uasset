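; BP_WinGame is a level trigger actor with two overlap boxes that respond only to BP_HeroCharacter, one for victory and one for game over.
; Box creates the VictoryScreen widget, shows the mouse cursor, switches the hero's PlayerHUDController to UI-only input and plays the victory cue.
; DedBox calls ShowPauseMenu on that controller, in place of a dedicated defeat screen, and plays the game over cue.
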(event `self.Box.OnComponentBeginOverlap`
  (params (OverlappedComponent :type "PrimitiveComponent Object Reference") (OtherActor :type "Actor Object Reference") (OtherComp :type "PrimitiveComponent Object Reference") (OtherBodyIndex :type Integer) (bFromSweep :type Boolean) (SweepResult :type "HitResult Structure (by ref)"))
  (bind _asbp_hero_character (cast `/Game/Character/BP_HeroCharacter` OtherActor))
  (bind _returnvalue (`|CreateWidget` "/Game/HUD/VictoryScreen.VictoryScreen_C"))
  (bind _playerhudcontroller (`HeroCharacter.playerHUDController` _asbp_hero_character))
  (set `PlayerController.bShowMouseCursor` true _playerhudcontroller)
  (`WidgetBlueprintLibrary.SetInputMode_UIOnlyEx` _playerhudcontroller _returnvalue)
  (`UserWidget.AddToViewport` _returnvalue 0)
  (`GameplayStatics.PlaySound2D` "/Game/Sounds/Victory_Cue.Victory_Cue" 1.0 1.0 0.0 null null))

(event `self.DedBox.OnComponentBeginOverlap`
  (params (OverlappedComponent :type "PrimitiveComponent Object Reference") (OtherActor :type "Actor Object Reference") (OtherComp :type "PrimitiveComponent Object Reference") (OtherBodyIndex :type Integer) (bFromSweep :type Boolean) (SweepResult :type "HitResult Structure (by ref)"))
  (bind _asbp_hero_character (cast `/Game/Character/BP_HeroCharacter` OtherActor))
  (`MainPlayerController.ShowPauseMenu` (`HeroCharacter.playerHUDController` _asbp_hero_character))
  (`GameplayStatics.PlaySound2D` "/Game/Sounds/Game_Over_Cue.Game_Over_Cue" 1.0 1.0 0.0 null null))

(fn `UserConstructionScript`)